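; Pillar flame actor that makes its fire light flicker.
; From BeginPlay, it randomly plays one of two flame intensity timelines and picks again whenever one finishes, forming an endless, varied loop.
; Each timeline update passes its curve value to 火焰闪烁 (flame flicker), which multiplies it by BaseIntensity to set the FireLight intensity, with no Tick logic.
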(event Custom|timeline1
  (bind _flameintensity (Timeline|FlameIntensity_1 PlayFromStart)
    (:Update
      (CallFunction|火焰闪烁 _flameintensity))
    (:Finished
      (CallFunction|ChooseTimeline))))

(event Custom|timeline2
  (bind _flameintensity (Timeline|FlameIntensity_2 PlayFromStart)
    (:Update
      (CallFunction|火焰闪烁 _flameintensity))
    (:Finished
      (CallFunction|ChooseTimeline))))

(event Custom|ChooseTimeline
  (switch int (Math|Random|RandomIntegerinRange 0 1)
    (:Default
      (CallFunction|Timeline1))
    (:0
      (CallFunction|Timeline1))
    (:1
      (CallFunction|Timeline2))))

(event EventBeginPlay
  (CallFunction|ChooseTimeline))

(event Collision|EventActorBeginOverlap
  (params (OtherActor :type Actor%20Object%20Reference)))

(event EventTick
  (params (DeltaSeconds :type Float%20%28single-precision%29)))

(fn ConstructionScript)

(fn 火焰闪烁
  (params (Intensity :type Float%20%28double-precision%29))
  (Rendering|Components|Light|SetIntensity (Variables|Default|GetFireLight) (* Intensity (Variables|Default|GetBaseIntensity))))