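; BP_FadeActor is a mesh actor that fades out and back in through FadeOut and Fadein events.
; Construction caches original materials and builds dynamic instances from the fade material list.
; FadeOut applies those instances and drives their Fade parameter by timeline, which Fadein reverses, restoring originals when finishing at full value.
; An optional flag makes the mesh block Visibility traces during fading, ignoring them after restoration, to control click-through.
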(event Collision|EventActorBeginOverlap
  (params (OtherActor :type Actor%20Object%20Reference)))

(event EventTick
  (params (DeltaSeconds :type Float%20%28single-precision%29)))

(event EventFadeOut
  (CallFunction|设置材质为动态实例)
  (bind _fadevalue (Timeline|Actor渐隐Timeline PlayFromStart)
    (:Update
      (for _array_element (Variables|Default|Get动态材质)
        (Rendering|Material|SetScalarParameterValue _array_element "Fade" _fadevalue :!class /Script/Engine.MaterialInstanceDynamic)
        (if (Variables|Default|Get阻挡可见性)
          (Collision|SetCollisionResponsetoChannel (Variables|Default|GetMesh) "ECC_Visibility" "ECR_Block") ; 区分楼梯是阻挡可见，可以点击上去，一些墙是忽略可见，点击就跑到后面
        )))
    (:Finished
      (if (>= _fadevalue 1.0)
        (CallFunction|重置材质为原始材质)
        (if (Variables|Default|Get阻挡可见性)
          (Collision|SetCollisionResponsetoChannel (Variables|Default|GetMesh) "ECC_Visibility" "ECR_Ignore"))
        (elif (<= _fadevalue 0.5)
          _)))))

(event EventFadein
  (bind _fadevalue (Timeline|Actor渐隐Timeline Reverse)
    (:Update
      (for _array_element (Variables|Default|Get动态材质)
        (Rendering|Material|SetScalarParameterValue _array_element "Fade" _fadevalue :!class /Script/Engine.MaterialInstanceDynamic)
        (if (Variables|Default|Get阻挡可见性)
          (Collision|SetCollisionResponsetoChannel (Variables|Default|GetMesh) "ECC_Visibility" "ECR_Block") ; 区分楼梯是阻挡可见，可以点击上去，一些墙是忽略可见，点击就跑到后面
        )))
    (:Finished
      (if (>= _fadevalue 1.0)
        (CallFunction|重置材质为原始材质)
        (if (Variables|Default|Get阻挡可见性)
          (Collision|SetCollisionResponsetoChannel (Variables|Default|GetMesh) "ECC_Visibility" "ECR_Ignore"))
        (elif (<= _fadevalue 0.5)
          _)))))

(fn ConstructionScript
  (Utilities|Array|Clear (Variables|Default|Get动态材质))
  (Variables|Default|Set原始材质 (Rendering|Material|GetMaterials (Variables|Default|GetMesh)))
  (for _array_element (Variables|Default|Get渐隐材质实例)
    (bind _returnvalue (Rendering|Material|CreateDynamicMaterialInstance _array_element "None" "None" :!class /Script/Engine.KismetMaterialLibrary)) ; 根据材质实例创建一个动态材质数组
    (Utilities|Array|AddUnique (Variables|Default|Get动态材质) _returnvalue)))

(fn 设置材质为动态实例
  (for (_array_element _array_index) (Variables|Default|Get动态材质)
    (Rendering|Material|SetMaterial (Variables|Default|GetMesh) _array_index _array_element)))

(fn 重置材质为原始材质
  (for (_array_element _array_index) (Variables|Default|Get原始材质)
    (Rendering|Material|SetMaterial (Variables|Default|GetMesh) _array_index _array_element)))