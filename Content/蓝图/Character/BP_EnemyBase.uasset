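; Base enemy character Blueprint that handles spawn scale-in, attack facing, death dissolve visuals and loot drops.
; BeginPlay scales the mesh via timeline, UpdateFacingTarget feeds a motion-warping target, and two timelines drive the Dissolve parameter on body and weapon materials.
; SpawnLoot rolls loot-tier items, then a looping timer spawns them one by one in an evenly spaced ring, setting effect actors to the enemy's level; the level-override branch is empty.
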(event Custom|SpawnLootItem
  (bind _lootitems (Variables|Default|GetLootItems))
  (bind _loopcount (Variables|Default|GetLoopCount))
  (bind _output (Utilities|Array|Get(acopy) _lootitems _loopcount))
  (bind (_lootclass _blootleveloverride) (Utilities|Struct|BreakLootItem _output))
  (if (< (Variables|Default|GetLoopCount) (Utilities|Array|Length (Variables|Default|GetLootItems)))
    (bind _returnvalue (Game|SpawnActorfromClass _lootclass (CallFunction|GetLootTransform (Variables|Default|GetLoopCount)) "AlwaysSpawn" "MultiplyWithRoot" 0 0))
    (bind _asaura_effect_actor (Utilities|Casting|CastToAuraEffectActor _returnvalue))
    (Variables|/Script/aura.AuraEffectActor|SetActorLevel _asaura_effect_actor (Math|Conversions|ToFloat(Integer) (Variables|Default|GetLevel)))
    (if _blootleveloverride
      _
      (else
        _))
    (Math|Integer|IncrementInt (Variables|Default|GetLoopCount))
    (else
      (Utilities|Time|ClearandInvalidateTimerbyHandle (Variables|Default|GetLoopTimer)))))

(event EventBeginPlay
  (bind _scaletrace (Timeline|SpawnTimeline Play)
    (:Update
      (Transformation|SetRelativeScale3D (Variables|Character|GetMesh) (Math|Vector|MakeVector _scaletrace _scaletrace _scaletrace)))))

(event Collision|EventActorBeginOverlap
  (params (OtherActor :type Actor%20Object%20Reference)))

(event EventTick
  (params (DeltaSeconds :type Float%20%28single-precision%29)))

(event EventStartDissolveTimeline
  (params (DynamicMaterialInstance :type Material%20Instance%20Dynamic%20Object%20Reference))
  (bind _溶解轨道 (Timeline|溶解Timeline Play)
    (:Update
      (Rendering|Material|SetScalarParameterValue DynamicMaterialInstance "Dissolve" _溶解轨道 :!class /Script/Engine.MaterialInstanceDynamic))))

(event EventWeaponStartDissolveTimeline
  (params (DynamicMaterialInstance :type Material%20Instance%20Dynamic%20Object%20Reference))
  (bind _溶解轨道 (Timeline|时间轴 Play)
    (:Update
      (Rendering|Material|SetScalarParameterValue DynamicMaterialInstance "Dissolve" _溶解轨道 :!class /Script/Engine.MaterialInstanceDynamic))))

(event EventUpdateFacingTarget
  (params (Target :type Vector%20%28by%20ref%29 :default "0, 0, 0"))
  (Class|MotionWarpingComponent|AddorUpdateWarpTargetfromLocation (Variables|Default|GetMotionWarping) "FacingTarget" Target))

(event EventSpawnLoot
  (bind _returnvalue (Class|AuraAbilitySystemLibrary|GetLootTiers))
  (Utilities|IsValid _returnvalue
    (:Is%20Valid
      (bind _returnvalue_2 (Class|LootTier|GetLootItems _returnvalue))
      (bind _output_get (Variables|Default|SetLootItems _returnvalue_2))
      (Variables|Default|SetLoopRotation (Class|AuraAbilitySystemLibrary|EvenlySpacedRotators (Transformation|GetActorForwardVector) (Math|Vector|VectorUp) 3.6e+02 (Utilities|Array|Length _output_get)))
      (Variables|Default|SetLoopCount 0)
      (bind _returnvalue_3 (Utilities|Time|SetTimerbyEvent (delegate Custom|SpawnLootItem) 0.1 true))
      (Variables|Default|SetLoopTimer _returnvalue_3)
      (CallFunction|SpawnLootItem))))

(fn ConstructionScript)

(fn GetLootTransform
  (params (LootCount :type Integer))
  (bind _looprotation (Variables|Default|GetLoopRotation))
  (bind _output (Utilities|Array|Get(acopy) _looprotation LootCount))
  (return (Math|Transform|MakeTransform (+ (* (Math|Vector|GetForwardVector _output) (Variables|Default|GetSpawnDistance)) (Transformation|GetActorLocation)) _output)))