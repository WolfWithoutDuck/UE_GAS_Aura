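; Enemy summon ability in which a shaman spawns random minions around the battlefield.
; It shuffles the spawn locations, plays a ground Niagara effect at each and starts the summon montage.
; On the montage's attack gameplay event, a delayed loop spawns one AI-controlled minion per location, slightly raised and facing the combat target.
; Each spawn increments the summoner's minion count, and each minion's OnDestroyed decrements it.
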(event Custom|OnDestroyed_事件
  (params (DestroyedActor :type Actor%20Object%20Reference))
  (Class|CombatInterface|IncrementMinionCount(Message) (Ability|GetAvatarActorfromActorInfo) -1))

(event Ability|EventActivateAbility
  (bind _returnvalue (Class|AuraSummonAbility|GetSpawnLocation))
  (bind _output_get (Variables|Default|Set生成位置 _returnvalue))
  (Utilities|Array|Shuffle _output_get)
  (for _array_element _output_get
    (Niagara|SpawnSystematLocation "/Game/Assets/Effects/Combat/NS_GroundSummon.NS_GroundSummon" _array_element))
  (|PlayMontageandWaitProxy "None" "/Game/Assets/Enemies/Shaman/Animations/AM_Shaman_Summon.AM_Shaman_Summon" 1.0 "None" true 1.0 0.0 false
    (:then
      (Ability|Tasks|WaitGameplayEvent "(TagName=\"Montage.Attack.1\")" 0
        (:EventReceived
          (bind _returnvalue_2 (Class|EnemyInterface|GetCombatTarget(Message) (Ability|GetAvatarActorfromActorInfo)))
          (if (< (Variables|Default|Get生成索引) (Utilities|Array|Length (Variables|Default|Get生成位置))) :!label _label
            (bind _returnvalue_3 (Game|SpawnActorfromClass (Class|AuraSummonAbility|GetRandomMinionClass) (Math|Transform|MakeTransform (+ (Utilities|Array|Get(acopy) (Variables|Default|Get生成位置) (Variables|Default|Get生成索引)) "0.000000,0.000000,70.000000") (Math|Rotator|FindLookatRotation (+ (Utilities|Array|Get(acopy) (Variables|Default|Get生成位置) (Variables|Default|Get生成索引)) "0.000000,0.000000,70.000000") (Transformation|GetActorLocation _returnvalue_2)) "1.000000,1.000000,1.000000") "AlwaysSpawn" "MultiplyWithRoot" 0 0))
            (Game|AssignOnDestroyed _returnvalue_3 (delegate Custom|OnDestroyed_事件))
            (Pawn|SpawnDefaultController _returnvalue_3)
            (Class|CombatInterface|IncrementMinionCount(Message) (Ability|GetAvatarActorfromActorInfo) 1)
            (Math|Integer|IncrementInt (Variables|Default|Get生成索引)
              (:%20%20
                (Utilities|FlowControl|Delay 0.2)
                (goto _label)))))))))

(event Ability|EventOnEndAbility
  (params (bWasCancelled :type Boolean)))