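; Slingshot projectile Blueprint for an enemy ability, with a rock mesh.
; BeginPlay picks random yaw, pitch and roll spin rates for a tumbling effect.
; The DeltaSeconds-scaled local rotation that would spin the mesh is disconnected from Tick and never runs, so this graph does not rotate the rock.
; The graph contains no movement or hit logic.
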(event EventBeginPlay
  (bind _returnvalue (Math|Random|RandomFloatinRange -5e+02 5e+02))
  (Variables|Default|SetYawRotation _returnvalue)
  (Variables|Default|SetPitchRotation _returnvalue)
  (Variables|Default|SetRollRotation _returnvalue))

(event Collision|EventActorBeginOverlap
  (params (OtherActor :type Actor%20Object%20Reference)))

(event EventTick
  (params (DeltaSeconds :type Float%20%28single-precision%29)))

(fn ConstructionScript)