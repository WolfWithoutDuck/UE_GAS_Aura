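; Enemy ranged attack gameplay ability that fires a projectile at the avatar's combat target.
; On activation it turns the avatar toward the target through interface messages, then plays a random montage from the avatar's tagged attack montages.
; The montage's gameplay event times the shot: the target location is re-read, a projectile spawns using the montage's socket tag, and the ability ends without stopping the montage.
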(event Ability|EventActivateAbility
  (bind _returnvalue (Ability|GetAvatarActorfromActorInfo))
  (bind _returnvalue_2 (Class|EnemyInterface|GetCombatTarget(Message) _returnvalue)) ; 获取战斗目标对象
  (Class|CombatInterface|UpdateFacingTarget(Message) _returnvalue (Transformation|GetActorLocation _returnvalue_2)) ; 朝向目标旋转
  (bind _returnvalue_3 (Class|CombatInterface|GetAttackMontages(Message) _returnvalue)) ; 获取当前所有的攻击蒙太奇
  (bind _output_get (Variables|Default|SetSelectedMontage (Class|AuraDamageGameplayAbility|GetRandomTaggedMontagefromArray _returnvalue_3)))
  (|PlayMontageandWaitProxy "None" (.Montage (Utilities|Struct|BreakTaggedMontage _output_get)) 1.0 "None" false 1.0 0.0 false
    (:then
      (Ability|Tasks|WaitGameplayEvent (.MontageTag (Utilities|Struct|BreakTaggedMontage _output_get)) 0 ; 攻击时机触发，近战直接造成伤害，远程生成投射物
        (:EventReceived
          (bind _returnvalue_4 (Class|EnemyInterface|GetCombatTarget(Message) (Ability|GetAvatarActorfromActorInfo))) ; 获取战斗目标对象
          (Class|AuraProjectileSpell|SpawnProjectile (Transformation|GetActorLocation _returnvalue_4) (.SocketTag (Utilities|Struct|BreakTaggedMontage _output_get)) false 0.0)
          (Ability|EndAbility))))))

(event Ability|EventOnEndAbility
  (params (bWasCancelled :type Boolean)))