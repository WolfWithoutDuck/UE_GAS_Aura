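; Gameplay ability for Arcane Shards, a magic-circle targeted spell that erupts shards around a point picked under the mouse.
; An input press spawns a point collection providing randomly rotated ground points, their count set by capped ability level, then plays the cast montage.
; The montage's gameplay event starts a looping timer that, per point, applies radial damage with pitched outward knockback, fires a GameplayCue and draws debug spheres.
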(event Custom|SpawnShards
  (if (< (Variables|Default|GetCount) (Variables|Default|GetNum%20Points))
    (CallFunction|保存技能生成位置)
    (CallFunction|获取技能范围内敌人Actor)
    (for _array_element (Variables|Default|GetOut%20Overlapping%20Actors)
      ;[1 1 1] 造成伤害
      (Class|AuraAbilitySystemLibrary|ApplyDamageEffect (Class|AuraDamageGameplayAbility|MakeDamageEffectParamsfromClassDefaults _array_element (Variables|Default|GetShardsSpawnsLocation) true (- (Transformation|GetActorLocation _array_element) (Variables|Default|GetShardsSpawnsLocation)) false "0, 0, 0" true 45.0)))
    (Math|Integer|IncrementInt (Variables|Default|GetCount)
      (:%20%20
        ;[1 1 1] 广播生成特效
        (Class|GameplayAbility|ExecuteGameplayCuewithParams "(TagName=\"GameplayCue.ArcaneShards\")" (Ability|GameplayCue|MakeGameplayCueParameters :Location (Variables|Default|GetShardsSpawnsLocation)))))
    (else
      (Utilities|Time|ClearandInvalidateTimerbyHandle (Variables|Default|GetShardSpawnTimer))
      (Utilities|FlowControl|Delay 0.1)
      (Actor|DestroyActor (Variables|Default|GetPointCollection)))))

(event Ability|EventActivateAbility
  (Variables|Default|SetNum%20Points (Math|Integer|Min(Integer) (Ability|GetAbilityLevel) (Variables|Default|GetMaxNumShards)))
  (Utilities|FlowControl|Sequence
    (:then_0
      (Class|PlayerInterface|ShowMagicCircle(Message) (Ability|GetAvatarActorfromActorInfo) 0))
    (:then_1
      (Ability|Tasks|WaitInputPress false
        (:OnPress
          (bind _datahandle (|TargetDataUnderMouse)
            (:ValidData
              ;[1 1 1] 获取当前特效生成落点
              (Variables|Default|SetHitLocation (.ImpactPoint (Collision|BreakHitResult (Ability|TargetData|GetHitResultfromTargetData _datahandle))))
              (bind _returnvalue (Game|SpawnActorfromClass "/Game/蓝图/AbilitySystem/Aura/Ability/Arcane/BP_PointCollection.BP_PointCollection_C" (Math|Transform|MakeTransform (Variables|Default|GetHitLocation) "0, 0, 0" "1.000000,1.000000,1.000000") "AlwaysSpawn" "MultiplyWithRoot" 0 0))
              (Variables|Default|SetPointCollection _returnvalue)
              (Variables|Default|SetGroundPoints (Class|PointCollection|GetGroundPoints (Variables|Default|GetPointCollection) (Variables|Default|GetHitLocation) (Variables|Default|GetNum%20Points) (Math|Random|RandomFloatinRange 0.0 3.6e+02)))
              ;[1 1 1] 朝向目标
              (Class|CombatInterface|UpdateFacingTarget(Message) (Ability|GetAvatarActorfromActorInfo) (Variables|Default|GetHitLocation))
              ;[1 1 1] 播放蒙太奇
              (|PlayMontageandWaitProxy "None" "/Game/Assets/Characters/Aura/Animations/Abilities/AM_Cast_ArcaneShards.AM_Cast_ArcaneShards" 1.0 "None" false 1.0 0.0 false
                (:then
                  (Ability|Tasks|WaitGameplayEvent "(TagName=\"Event.Montage.ArcanesShards\")" 0 true
                    (:EventReceived
                      (bind _returnvalue_2 (Utilities|Time|SetTimerbyEvent (delegate Custom|SpawnShards) (Variables|Default|GetShardSpawnDeltaTimer) true))
                      (Variables|Default|SetShardSpawnTimer _returnvalue_2)
                      (Class|PlayerInterface|HideMagicCircle(Message) (Ability|GetAvatarActorfromActorInfo))
                      (CallFunction|SpawnShards))))
                (:OnCompleted
                  (Ability|EndAbility))))))))))

(event Ability|EventOnEndAbility
  (params (bWasCancelled :type Boolean)))

(fn 保存技能生成位置
  (Variables|Default|SetShardsSpawnsLocation (Transformation|GetWorldLocation (Utilities|Array|Get(acopy) (Variables|Default|GetGroundPoints) (Variables|Default|GetCount)))))

(fn 获取技能范围内敌人Actor
  (bind _returnvalue (Ability|GetAvatarActorfromActorInfo))
  (Rendering|Debug|DrawDebugSphere (Variables|Default|GetShardsSpawnsLocation) (Variables|Default|GetRadialDamageInnerRadius) 12 "(R=1.000000,G=1.000000,B=1.000000,A=1.000000)" 3.0)
  (Rendering|Debug|DrawDebugSphere (Variables|Default|GetShardsSpawnsLocation) (Variables|Default|GetRadialDamageOuterRadius) 12 "(R=1.000000,G=0.230999,B=0.549229,A=1.000000)" 3.0)
  (bind _outoverlappingactors (Class|AuraAbilitySystemLibrary|GetLivePlayersWithinRadius _returnvalue (Utilities|Array|MakeArray _returnvalue) (Variables|Default|GetRadialDamageOuterRadius) (Variables|Default|GetShardsSpawnsLocation)))
  (Variables|Default|SetOut%20Overlapping%20Actors _outoverlappingactors))