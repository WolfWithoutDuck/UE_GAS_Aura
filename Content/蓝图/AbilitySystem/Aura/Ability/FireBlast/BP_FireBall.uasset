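; BP_FireBall is the Fire Blast ability projectile that flies out, returns to its ReturnToActor and explodes.
; On the server, StartOutgoingTimeline drives two timeline lerps: forward by TravelDistance, then back toward that actor's current location.
; Within ExplodeDistance it calls OnHit, applies radial ExplosionDamage through the owning damage ability to nearby live players except its owner, draws debug spheres, and destroys itself.
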(event EventBeginPlay)

(event Collision|EventActorBeginOverlap
  (params (OtherActor :type Actor%20Object%20Reference)))

(event EventTick
  (params (DeltaSeconds :type Float%20%28single-precision%29)))

(event EventStartOutgoingTimeline
  (bind _returnvalue (Transformation|GetActorLocation))
  (Networking|SwitchHasAuthority
    (:Authority
      ;[1 1 1] 初始化投射物位置
      (Variables|Default|SetInitialLocation (Transformation|GetActorLocation))
      (Variables|Default|SetApexLocation (+ (* (Transformation|GetActorForwardVector) (Variables|Default|GetTravelDistance)) (Variables|Default|GetInitialLocation)))
      (bind _outgoingtrace (Timeline|OutgoingTimeline Play)
        (:Update
          (Transformation|SetActorLocation (Math|Vector|Lerp(Vector) (Variables|Default|GetInitialLocation) (Variables|Default|GetApexLocation) _outgoingtrace) false false))
        (:Finished
          (bind _outgoingtrace_2 (Timeline|returnTimeline Play)
            (:Update
              (Transformation|SetActorLocation (Math|Vector|Lerp(Vector) (Variables|Default|GetApexLocation) (Transformation|GetActorLocation (Variables|Default|GetReturnToActor)) _outgoingtrace_2) false false)
              (if (CallFunction|检测投射物离人物距离)
                (Class|AuraProjectile|OnHit)
                (bind _outoverlappingactors (Class|AuraAbilitySystemLibrary|GetLivePlayersWithinRadius self (Utilities|Array|MakeArray (Components|GetOwner)) 3e+02 (Transformation|GetActorLocation)))
                (bind _output_get (Variables|Default|SetOut%20Overlapping%20Actors _outoverlappingactors))
                (for _array_element _output_get
                  (Variables|Default|SetDamageEffect (Class|AuraDamageGameplayAbility|MakeDamageEffectParamsfromClassDefaults (Variables|Default|GetOwnerDamageAbility) _array_element "0, 0, 0" false "0, 0, 0" false "0, 0, 0" false 0.0))
                  (Class|AuraAbilitySystemLibrary|SetDamageEffectParam (Variables|Default|GetDamageEffect) (Variables|Default|GetExplosionDamage))
                  (Class|AuraAbilitySystemLibrary|SetIsRadialDamageEffectParam (Variables|Default|GetDamageEffect) true 3e+02 5e+01 _returnvalue)
                  (Rendering|Debug|DrawDebugSphere _returnvalue 3e+02 12 "(R=1.000000,G=0.123204,B=0.471354,A=1.000000)" 3.0)
                  (Class|AuraAbilitySystemLibrary|ApplyDamageEffect (Variables|Default|GetDamageEffect)))
                (Actor|DestroyActor)))))))))

(fn ConstructionScript)

(fn 检测投射物离人物距离
  (return (<= (Math|Vector|VectorLength (- (Transformation|GetActorLocation) (Transformation|GetActorLocation (Variables|Default|GetReturnToActor)))) (Variables|Default|GetExplodeDistance))))