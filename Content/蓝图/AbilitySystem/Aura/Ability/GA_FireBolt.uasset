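; GA_FireBolt is the Aura fire bolt gameplay ability, which casts a projectile at the location under the mouse.
; On valid target data, it turns the avatar toward the hit location through CombatInterface and plays the cast montage.
; A montage-driven gameplay event tag times the projectile spawn to the animation.
; The ability ends with authority right after spawning, or whenever the montage completes, is interrupted or is cancelled.
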(event Ability|EventActivateAbility
  (bind _datahandle (|TargetDataUnderMouse)
    (:ValidData
      (Variables|Default|Set投射物目标位置 (.Location (Collision|BreakHitResult (Ability|TargetData|GetHitResultfromTargetData _datahandle))))
      (bind _ascombat_interface (Utilities|Casting|CastToCombatInterface (Ability|GetAvatarActorfromActorInfo)))
      (Class|CombatInterface|UpdateFacingTarget _ascombat_interface (Variables|Default|Get投射物目标位置)) ; 根据投射物的位置，调用旋转事件，朝向目标
      (|PlayMontageandWaitProxy "None" "/Game/Assets/Characters/Aura/Animations/Abilities/AM_Cast_FireBolt.AM_Cast_FireBolt" 1.0 "None" true 1.0 0.0 false
        (:then
          (Ability|Tasks|WaitGameplayEvent "(TagName=\"Event.Montage.FireBolt\")" 0 ; 等待蒙太奇上的动画Tag事件触发，然后指定动画动作生成投射物火球
            (:EventReceived
              (Class|AuraProjectileSpell|SpawnProjectile (Variables|Default|Get投射物目标位置))
              (if (Ability|HasAuthority (Ability|GetAvatarActorfromActorInfo))
                (Ability|EndAbility)))))
        (:OnCompleted
          (Ability|EndAbility :!label _label))
        (:OnInterrupted
          (goto _label))
        (:OnCancelled
          (goto _label))))))

(event Ability|EventOnEndAbility
  (params (bWasCancelled :type Boolean)))