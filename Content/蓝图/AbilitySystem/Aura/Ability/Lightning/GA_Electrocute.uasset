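; Channeled chain lightning ability for the Aura character, aimed at the target under the mouse.
; A montage event locks movement and adds looping shock cues on the hit target (or caster on a miss), chaining to additional enemies.
; A looping timer commits cost and applies set-by-caller damage.
; Input release (padded to a minimum cast time), failed cost or primary-target death ends it, while chained deaths drop only their arc.
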(event Custom|DamageAndCost
  (bind _returnvalue (Ability|CommitAbilityCost false))
  (if _returnvalue
    (if (Variables|Default|Get第一个目标是否实现战斗接口)
      (CallFunction|添加伤害))
    (else
      (CallFunction|清除计时器结束能力))))

(event Ability|EventActivateAbility
  (CallFunction|确保继承战斗接口)
  (bind _asbp_aura_character (Utilities|Casting|CastToBP_AuraCharacter (Ability|GetAvatarActorfromActorInfo)))
  ;[1 1 1] 存储玩家信息
  (Variables|Default|SetAs%20BP%20Aura%20Character _asbp_aura_character)
  (bind _datahandle (|TargetDataUnderMouse)
    (:ValidData
      (Class|AuraBeamSpell|StoreMouseDataInfo (Ability|TargetData|GetHitResultfromTargetData _datahandle))
      (Class|AuraBeamSpell|StoreOwnerVariables)
      (Utilities|FlowControl|Sequence
        (:then_0
          (Variables|/Script/Engine.PlayerController|SetbShowMouseCursor (Variables|Default|GetOwnerPlayerController) false)
          (Class|CombatInterface|UpdateFacingTarget(Message) (Ability|GetAvatarActorfromActorInfo) (Variables|Default|GetMouseHitLocation)) ; 蓝图基类实现了
          (GameplayCue|ExecuteGameplayCue :GameplayCueTag "(TagName=\"GameplayCue.ShockBurst\")")
          (|PlayMontageandWaitProxy "None" (Variables|Default|GetMontage_Electrocute) 1.0 "None" false 1.0 0.0 false
            (:then
              (Ability|Tasks|WaitGameplayEvent "(TagName=\"Event.Montage.Electrocute\")" 0 true
                (:EventReceived
                  (CallFunction|持续吟唱循环)
                  (CallFunction|生成电弧)
                  (bind _returnvalue (Utilities|Time|SetTimerbyEvent (delegate Custom|DamageAndCost) (Variables|Default|GetDamageDeltaTime) true))
                  (Variables|Default|SetDamageAndCostTimer _returnvalue))))))
        (:then_1
          ;[1 1 1] 确保按下之后，松开有个最小延迟，保证技能前摇放出来
          (bind _timeheld (Ability|Tasks|WaitInputRelease false)
            (:OnRelease
              (Variables|Default|SetTime%20Held _timeheld)
              (if (< (Variables|Default|GetTime%20Held) (Variables|Default|GetMinSpellTime))
                (Ability|HasAuthority
                  (:True
                    (Utilities|FlowControl|Delay (- (Variables|Default|GetMinSpellTime) (Variables|Default|GetTime%20Held)))
                    (CallFunction|清除计时器结束能力 :!label _label))
                  (:False
                    (CallFunction|准备结束能力)))
                (else
                  (goto _label))))))))))

(event Ability|EventOnEndAbility
  (params (bWasCancelled :type Boolean)))

(event EventPrimaryTargetDied
  (params (DeadActor :type Actor%20Object%20Reference))
  ;[1 1 1] 主要怪物死亡
  (GameplayCue|RemoveGameplayCueOnActor(Looping) DeadActor "(TagName=\"GameplayCue.ShockLoop\")" (Variables|Default|GetFirstTargetCueParameters))
  (CallFunction|清除计时器结束能力))

(event EventAdditionalTargetDied
  (params (DeadActor :type Actor%20Object%20Reference))
  ;[1 1 1] 连锁的怪物死亡
  (CallFunction|从映射中移除电弧特效Cue DeadActor)
  (Utilities|Array|RemoveItem (Variables|Default|GetOut%20Additional%20Targets) DeadActor))

(fn 确保继承战斗接口
  (if (not (Utilities|DoesObjectImplementInterface (Ability|GetAvatarActorfromActorInfo) "/Script/aura.CombatInterface"))
    (Ability|EndAbility)))

(fn 准备结束能力
  (bind _mousehitactor (Variables|Default|GetMouseHitActor))
  (Variables|/Script/Engine.PlayerController|SetbShowMouseCursor (Variables|Default|GetOwnerPlayerController) true)
  (Class|CombatInterface|SetinShockLoop(Message) (Ability|GetAvatarActorfromActorInfo) false)
  (Pawn|Components|CharacterMovement|SetMovementMode (Variables|/Script/Engine.Character|GetCharacterMovement (Variables|Default|GetOwnerCharacter)) "MOVE_Walking" 0)
  (if (Variables|Default|Get第一个目标是否实现战斗接口)
    (Class|CombatInterface|SetIsBeingShocked(Message) (Variables|Default|GetCueTarget) false)
    (GameplayCue|RemoveGameplayCueOnActor(Looping) (Variables|Default|GetCueTarget) "(TagName=\"GameplayCue.ShockLoop\")" (Variables|Default|GetFirstTargetCueParameters))
    (Ability|HasAuthority
      (:True
        (Utilities|IsValid _mousehitactor
          (:Is%20Valid
            (Class|AuraAbilitySystemLibrary|ApplyDamageEffect (Class|AuraDamageGameplayAbility|MakeDamageEffectParamsfromClassDefaults _mousehitactor "0, 0, 0" false "0, 0, 0" false "0, 0, 0" false 0.0)))))
      (:False
        _))
    (for _array_element (Variables|Default|GetOut%20Additional%20Targets)
      (Class|CombatInterface|SetIsBeingShocked(Message) _array_element false)
      (CallFunction|从映射中移除电弧特效Cue _array_element)
      (Ability|HasAuthority
        (:True
          (Class|AuraAbilitySystemLibrary|ApplyDamageEffect (Class|AuraDamageGameplayAbility|MakeDamageEffectParamsfromClassDefaults _array_element "0, 0, 0" false "0, 0, 0" false "0, 0, 0" false 0.0)))))
    (else
      (GameplayCue|RemoveGameplayCueOnActor(Looping) (Variables|Default|GetCueTarget) "(TagName=\"GameplayCue.ShockLoop\")" (Variables|Default|GetFirstTargetCueParameters)))))

(fn 持续吟唱循环
  (Class|CombatInterface|SetinShockLoop(Message) (Ability|GetAvatarActorfromActorInfo) true)
  (Pawn|Components|CharacterMovement|DisableMovement (Variables|/Script/Engine.Character|GetCharacterMovement (Variables|Default|GetOwnerCharacter))))

(fn 生成电弧
  (Class|AuraBeamSpell|TraceFirstTarget (Variables|Default|GetMouseHitLocation))
  (bind _returnvalue (Class|CombatInterface|GetWeapon(Message) (Variables|Default|GetOwnerCharacter)))
  (Variables|Default|SetFirstTargetCueParameters (Ability|GameplayCue|MakeGameplayCueParameters :Location (Variables|Default|GetMouseHitLocation) :SourceObject (Variables|Default|GetMouseHitActor) :TargetAttachComponent _returnvalue))
  (bind _output_get (Variables|Default|Set第一个目标是否实现战斗接口 (Utilities|DoesObjectImplementInterface (Variables|Default|GetMouseHitActor) "/Script/aura.CombatInterface")))
  ;[1 1 1] 检查是否击中敌人，击中敌人电弧特效Cue的拥有者是敌人，击中地板等，电弧特效的Cue的拥有者是角色自己
  (if _output_get ; 电弧击中是否击中敌人
    (Variables|Default|SetCueTarget (Variables|Default|GetMouseHitActor))
    (else
      (Variables|Default|SetCueTarget (Ability|GetAvatarActorfromActorInfo))))
  (GameplayCue|AddGameplayCueOnActor(Looping) (Variables|Default|GetCueTarget) "(TagName=\"GameplayCue.ShockLoop\")" (Variables|Default|GetFirstTargetCueParameters))
  (if (Variables|Default|Get第一个目标是否实现战斗接口)
    (Class|CombatInterface|SetIsBeingShocked(Message) (Variables|Default|GetCueTarget) true)
    (bind _outadditionaltargets (Class|AuraBeamSpell|StoreAdditionalTargets))
    (bind _output_get_2 (Variables|Default|SetOut%20Additional%20Targets _outadditionaltargets))
    (for _array_element _output_get_2
      (CallFunction|连接电弧到敌人 _array_element)
      (Class|CombatInterface|SetIsBeingShocked(Message) _array_element true))))

(fn 连接电弧到敌人
  (params (AdditionalTarget :type Actor%20Object%20Reference))
  (bind _output_get (LocalVariables|SetTargetActor AdditionalTarget))
  (Utilities|Map|Add (Variables|Default|GetActor到Cue参数映射) _output_get (Ability|GameplayCue|MakeGameplayCueParameters :Location (Transformation|GetActorLocation (LocalVariables|GetTargetActor)) :SourceObject (LocalVariables|GetTargetActor) :TargetAttachComponent (Variables|/Script/Engine.Actor|GetRootComponent (Variables|Default|GetMouseHitActor))))
  (GameplayCue|AddGameplayCueOnActor(Looping) (LocalVariables|GetTargetActor) "(TagName=\"GameplayCue.ShockLoop\")" (Ability|GameplayCue|MakeGameplayCueParameters :Location (Transformation|GetActorLocation (LocalVariables|GetTargetActor)) :SourceObject (LocalVariables|GetTargetActor) :TargetAttachComponent (Variables|/Script/Engine.Actor|GetRootComponent (Variables|Default|GetMouseHitActor))))
  (return))

(fn 从映射中移除电弧特效Cue
  (params (target :type Actor%20Object%20Reference))
  (bind _actor到cue参数映射 (Variables|Default|GetActor到Cue参数映射))
  (bind (_value _returnvalue) (Utilities|Map|Find _actor到cue参数映射 target))
  (if _returnvalue
    (GameplayCue|RemoveGameplayCueOnActor(Looping) target "(TagName=\"GameplayCue.ShockLoop\")" _value)))

(fn 添加伤害
  (CallFunction|给一个Actor添加伤害 (Variables|Default|GetMouseHitActor))
  (for _array_element (Variables|Default|GetOut%20Additional%20Targets)
    (CallFunction|给一个Actor添加伤害 _array_element)))

(fn 给一个Actor添加伤害
  (params (Actor :type Actor%20Object%20Reference))
  (bind _returnvalue (Ability|GetAbilitySystemComponentfromActorInfo))
  (Utilities|IsValid Actor
    (:Is%20Valid
      (Utilities|IsValid _returnvalue
        (:Is%20Valid
          (LocalVariables|SetDamageEffectSpec (GameplayEffects|MakeOutgoingSpec _returnvalue (Variables|Default|GetDamageEffectClass) (Math|Conversions|ToFloat(Integer) (Ability|GetAbilityLevel)) (GameplayEffects|MakeEffectContext _returnvalue)))
          (bind _returnvalue_2 (Class|AuraBeamSpell|GetCauseDamage))
          (bind _keys (Utilities|Map|Keys _returnvalue_2))
          (for _array_element _keys
            (if (.ReturnValue (Utilities|Map|Find _returnvalue_2 _array_element))
              (Ability|GameplayEffect|AssignTagSetbyCallerMagnitude (LocalVariables|GetDamageEffectSpec) _array_element (.Value (Utilities|Map|Find _returnvalue_2 _array_element)))))
          (GameplayEffects|ApplyGameplayEffectSpecToSelf (Ability|GetAbilitySystemComponent Actor) (LocalVariables|GetDamageEffectSpec)))))))

(fn 清除计时器结束能力
  (bind _damageandcosttimer (Variables|Default|GetDamageAndCostTimer))
  (if (Utilities|Time|IsValidTimerHandle _damageandcosttimer)
    (Utilities|Time|ClearandInvalidateTimerbyHandle _damageandcosttimer))
  (CallFunction|准备结束能力)
  (Ability|CommitAbilityCooldown false)
  (Utilities|Array|Clear (Variables|Default|GetOut%20Additional%20Targets))
  (Utilities|Array|Clear (Variables|Default|GetOut%20Additional%20Targets))
  (Variables|Default|SetMouseHitActor 0)
  (Variables|Default|Set第一个目标是否实现战斗接口 false)
  (Variables|Default|SetTime%20Held 0.0)
  (Ability|EndAbility))