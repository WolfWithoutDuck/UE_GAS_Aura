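; BP_AuraMainMenu is the main menu scene actor that starts the menu and animates its magical backdrop.
; On BeginPlay it plays the menu music, adds WBP_MainMenu to the viewport, switches to UI-only input and shows the cursor.
; Each Tick, a timer that resets after one sine period bobs the fire bolt Niagara effect around its starting location, while the magic circle decal rotates at a configurable rate.
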(event EventBeginPlay
  (bind _returnvalue (Game|GetPlayerController 0))
  (Variables|Default|SetFireBoltLocation (Transformation|GetWorldLocation (Variables|Default|GetNiagara)))
  (Audio|PlaySound2D "/Game/Assets/Sounds/Music/Music_MainMenu.Music_MainMenu" 1.0 1.0 0.0 0 0)
  (bind _returnvalue_2 (UserInterface|CreateWidget "/Game/蓝图/UI/MainMenu/WBP_MainMenu.WBP_MainMenu_C"))
  (UserInterface|Viewport|AddtoViewport _returnvalue_2 0)
  (Input|SetInputModeUIOnly _returnvalue 0 "DoNotLock" false)
  (Variables|/Script/Engine.PlayerController|SetbShowMouseCursor _returnvalue true))

(event Collision|EventActorBeginOverlap
  (params (OtherActor :type Actor%20Object%20Reference)))

(event EventTick
  (params (DeltaSeconds :type Float%20%28single-precision%29))
  (CallFunction|UpdateTimer DeltaSeconds)
  (Transformation|SetWorldLocation (Variables|Default|GetNiagara) (+ (Variables|Default|GetFireBoltLocation) (Math|Vector|MakeVector 0.0 0.0 (* (Math|Trig|Sin(Radians) (Variables|Default|GetTime)) (Variables|Default|GetAmplitude)))) false false)
  (Transformation|AddLocalRotation (Variables|Default|Get魔法阵贴花) (Math|Rotator|MakeRotator (* (Utilities|Time|GetWorldDeltaSeconds) (Variables|Default|GetMagicCircleRotationRate)) 0.0 0.0) false false))

(fn ConstructionScript)

(fn UpdateTimer
  (params (A :type Float%20%28double-precision%29))
  (bind _output_get (Variables|Default|SetTime (+ A (* (Variables|Default|GetTime) 1.0))))
  (if (> _output_get 6.28)
    (Variables|Default|SetTime 0.0)))